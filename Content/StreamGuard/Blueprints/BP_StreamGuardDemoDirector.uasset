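; StreamGuard demo director that drives throttled streaming of a list of district levels.
; On BeginPlay it applies its budget for concurrent loads and per-frame activation time, then sets the starting throttle and board visibility.
; Its functions queue loads or unloads for all districts, toggle throttling, and switch between hardcoded tight and loose budgets.
; Turning the throttle on reapplies the configured budget, replacing either preset.
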(event `self.ReceiveBeginPlay`
  (bind (_maxconcurrentloads _maxactivationmsperframe) (break `StreamGuardBudget` (`self.Budget`)))
  (`StreamGuardStatics.SetMaxConcurrentLoads` _maxconcurrentloads)
  (`StreamGuardStatics.SetMaxActivationMsPerFrame` _maxactivationmsperframe)
  (`StreamGuardStatics.SetThrottleEnabled` (`self.ThrottleAtStart`))
  (`StreamGuardStatics.SetShowBoard` (`self.ShowBoardAtStart`)))

(fn `BudgetLoose`
  (`StreamGuardStatics.SetMaxConcurrentLoads` 4)
  (`StreamGuardStatics.SetMaxActivationMsPerFrame` 8.0))

(fn `BudgetTight`
  (`StreamGuardStatics.SetMaxConcurrentLoads` 1)
  (`StreamGuardStatics.SetMaxActivationMsPerFrame` 1.0))

(fn `LoadAllDistricts`
  (for _array_element (`self.Districts`)
    (`StreamGuardStatics.RequestLevelLoad` _array_element)))

(fn `ThrottleOff`
  (`StreamGuardStatics.SetThrottleEnabled` false))

(fn `ThrottleOn`
  (bind (_maxconcurrentloads _maxactivationmsperframe) (break `StreamGuardBudget` (`self.Budget`)))
  (`StreamGuardStatics.SetMaxConcurrentLoads` _maxconcurrentloads)
  (`StreamGuardStatics.SetMaxActivationMsPerFrame` _maxactivationmsperframe)
  (`StreamGuardStatics.SetThrottleEnabled` true))

(fn `UnloadAllDistricts`
  (for _array_element (`self.Districts`)
    (`StreamGuardStatics.RequestLevelUnload` _array_element)))

(fn `UserConstructionScript`)