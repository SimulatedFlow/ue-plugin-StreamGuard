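; BP_StreamGuardDemoPawn is a StreamGuard demo pawn that moves along a circular route around the world origin while Driving is true.
; Tick accumulates RouteTime and converts it through RoutePeriod into an angle, placing the pawn at RouteRadius and RouteHeight.
; The same position feeds a look-at rotation, so the pawn always faces the origin.
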(event `self.ReceiveTick`
  (params (DeltaSeconds :type "Float (single-precision)"))
  (bind _routeradius (`self.RouteRadius`))
  (bind _returnvalue (+ (`self.RouteTime`) DeltaSeconds))
  (bind _returnvalue_2 (* 360.0 (/ _returnvalue (`self.RoutePeriod`))))
  (bind _returnvalue_3 (`KismetMathLibrary.MakeVector` (* _routeradius (`KismetMathLibrary.DegCos` _returnvalue_2)) (* _routeradius (`KismetMathLibrary.DegSin` _returnvalue_2)) (`self.RouteHeight`)))
  (if (`self.Driving`)
    (set `self.RouteTime` _returnvalue)
    (`self.K2_SetActorLocationAndRotation` _returnvalue_3 (`KismetMathLibrary.FindLookAtRotation` _returnvalue_3 (`KismetMathLibrary.MakeVector` 0.0)))))

(fn `UserConstructionScript`)